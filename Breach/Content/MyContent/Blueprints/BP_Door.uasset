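; BP_Door is a hinged door that the first-person player toggles when in range, with optional locking.
; The first overlap with PlayerActivateVolume binds the toggle to the character's IsUsing event, while overlaps track range.
; Separate timelines swing DoorMesh open and closed, or a locked door shows an onscreen message.
; InGameEvent can unlock flagged doors, announcing it and creating waypoint "B" through FirstPersonGameMode, which is removed when opening finishes.
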(event OnComponentBeginOverlap(PlayerActivateVolume)
  (params (OverlappedComponent :type Primitive%20Component%20Object%20Reference) (OtherActor :type Actor%20Object%20Reference) (OtherComp :type Primitive%20Component%20Object%20Reference) (OtherBodyIndex :type Integer) (bFromSweep :type Boolean) (SweepResult :type Hit%20Result%20Structure%20%28by%20ref%29))
  (bind _asfirst_person_character (Utilities|Casting|CastToFirstPersonCharacter OtherActor))
  (Variables|Default|SetPlayerInRange true)
  (if (Variables|Default|GetFirstCollision)
    (EventDispatchers|BindEventtoIsUsing _asfirst_person_character (delegate Custom|ToggleUnlockedDoor))
    (Variables|Default|SetFirstCollision false)))

(event OnComponentEndOverlap(PlayerActivateVolume)
  (params (OverlappedComponent :type Primitive%20Component%20Object%20Reference) (OtherActor :type Actor%20Object%20Reference) (OtherComp :type Primitive%20Component%20Object%20Reference) (OtherBodyIndex :type Integer))
  (Utilities|Casting|CastToFirstPersonCharacter OtherActor)
  (Variables|Default|SetPlayerInRange false))

(event Custom|CloseDoor
  (bind _doortrack (Timeline|DoorClose PlayFromStart)
    (:Update
      (Transformation|SetRelativeRotation (Variables|Default|GetDoorMesh) (Math|Rotator|MakeRotator 0.0 0.0 (Math|Float|Lerp 9e+01 0.0 _doortrack)) false false))
    (:Finished
      (Variables|Default|SetIsOpen false))))

(event Custom|OpenDoor
  (bind _doortrack (Timeline|DoorOpening PlayFromStart)
    (:Update
      (Transformation|SetRelativeRotation (Variables|Default|GetDoorMesh) (Math|Rotator|MakeRotator 0.0 0.0 (Math|Float|Lerp 0.0 9e+01 _doortrack)) false false))
    (:Finished
      (Variables|Default|SetIsOpen true)
      (bind _asfirst_person_game_mode (Utilities|Casting|CastToFirstPersonGameMode (Game|GetGameMode))
        (:then
          (Development|PrintString "Cast to FirstPErsonGameMode successfull!!!!!")
          (Default|RemoveWaypoint _asfirst_person_game_mode "B"))
        (:CastFailed
          (Development|PrintString "Cast to FirstPErsonGameMode has failed"))))))

(event Custom|ToggleUnlockedDoor
  (if (Variables|Default|GetPlayerInRange)
    (if (not (Variables|Default|GetIsLocked))
      (CallFunction|ToggleDoor)
      (else
        (bind _asfirst_person_game_mode (Utilities|Casting|CastToFirstPersonGameMode (Game|GetGameMode)))
        (Default|CallChangeOnscreenMessage _asfirst_person_game_mode "Door is locked" 2.0)))))

(event EventBeginPlay)

(event Collision|EventActorBeginOverlap
  (params (OtherActor :type Actor%20Object%20Reference)))

(event EventInGameEvent
  (if (Variables|Default|GetUnlocksOnEvent)
    (Variables|Default|SetIsLocked false)
    (bind _asfirst_person_game_mode (Utilities|Casting|CastToFirstPersonGameMode (Game|GetGameMode)))
    (Default|CallChangeOnscreenMessage _asfirst_person_game_mode "A door has been unlocked" 2.0)
    (bind _asfirst_person_game_mode_2 (Utilities|Casting|CastToFirstPersonGameMode (Game|GetGameMode)))
    (Default|CreateWaypoint _asfirst_person_game_mode_2 self "B")))

(event EventTick
  (params (DeltaSeconds :type Float%20%28single-precision%29)))

(fn ConstructionScript)

(fn ToggleDoor
  (if (Variables|Default|GetIsOpen)
    (CallFunction|CloseDoor)
    (else
      (CallFunction|OpenDoor)))
  (Variables|Default|SetIsOpen (not (Variables|Default|GetIsOpen))))