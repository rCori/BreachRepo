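; Area spawner that, when triggered by InGameEvent, spawns SpawnCount enemies at random positions and yaws within the SpawnArea bounds.
; Each spawned enemy gets an AI controller and starts aware of the player.
; With CompletionIsEvent set, enemy deaths count down CurrentAlive, firing InGameEvent on GenericCompletedEvent targets at zero to chain events.
; CurrentAlive starts at SpawnCount, so spawns blocked by collision still count as alive.
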(event Custom|TriggerAllKilledEvent
  ;[1 1 1] Will be called when all enemies are killed if an even is assigned to GenericEventAllKilled
  (if (Variables|Default|GetCompletionIsEvent)
    (bind _result (Math|Integer|DecrementInt (Variables|Default|GetCurrentAlive))
      (:%20%20
        (if (== _result 0)
          (for _array_element (Variables|Default|GetGenericCompletedEvent)
            (bind _asgeneric_in_game_event (Utilities|Casting|CastToGenericInGameEvent _array_element))
            (Default|InGameEvent _asgeneric_in_game_event)))))))

(event EventBeginPlay
  (Variables|Default|SetCurrentAlive (Variables|Default|GetSpawnCount)))

(event Collision|EventActorBeginOverlap
  (params (OtherActor :type Actor%20Object%20Reference)))

(event EventTick
  (params (DeltaSeconds :type Float%20%28single-precision%29)))

(event EventInGameEvent
  (CallFunction|SpawnAllCharactersinArea))

(fn ConstructionScript)

(fn SpawnAllCharactersinArea
  (bind _spawnarea (Variables|Default|GetSpawnArea))
  (bind (_origin _boxextent) (Collision|GetComponentBounds _spawnarea))
  (for _index (range 1 (Variables|Default|GetSpawnCount))
    (bind _returnvalue (Game|SpawnActorfromClass "/Game/EnemyCharacter/Blueprints/BP_EnemyCharacter.BP_EnemyCharacter_C" (Math|Transform|MakeTransform (+ _origin (Math|Vector|MakeVector (* (.x _boxextent) (Math|Random|RandomFloatinRange -1.0 1.0)) (* (.y _boxextent) (Math|Random|RandomFloatinRange -1.0 1.0)) (* (.z _boxextent) (Math|Random|RandomFloatinRange -1.0 1.0)))) (Math|Rotator|MakeRotator 0.0 0.0 (Math|Random|RandomFloatinRange 0.0 3.6e+02)) "1,1,1") "AdjustIfPossibleButDontSpawnIfColliding" 0 0))
    (Utilities|IsValid _returnvalue
      (:Is%20Valid
        (if (Variables|Default|GetCompletionIsEvent)
          (EventDispatchers|BindEventtoEnemyDead _returnvalue (EventDispatchers|CreateEvent :!event Custom|TriggerAllKilledEvent)))
        (Variables|/Script/Engine.Pawn|SetAIControllerClass _returnvalue "/Game/EnemyCharacter/Blueprints/EnemyAI/EnemyAIController.EnemyAIController_C")
        (Pawn|SpawnDefaultController _returnvalue)
        (Default|InitializeAwareOfPlayer _returnvalue)))))