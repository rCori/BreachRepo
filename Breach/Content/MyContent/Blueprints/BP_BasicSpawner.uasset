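; BP_BasicSpawner is an event-triggered spawner that places a group of AI enemies at offsets from its root.
; InGameEvent spawns a BP_EnemyCharacter with BT_EnemyAI at each location, initialized either player-aware or with index-matched trigger volumes and movement splines.
; When completion is an event, it binds to each enemy's death, counting down to fire InGameEvent on GenericCompletedEvent, allowing events to be chained.
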(event Custom|TriggerAllKilledEvent
  ;[1 1 1] Will be called when all enemies are killed if an even is assigned to GenericEventAllKilled
  (if (Variables|Default|GetCompletionIsEvent)
    (bind _result (Math|Integer|DecrementInt (Variables|Default|GetCurrentAlive))
      (:%20%20
        (if (== _result 0)
          (bind _asgeneric_in_game_event (Utilities|Casting|CastToGenericInGameEvent (Variables|Default|GetGenericCompletedEvent)))
          (Default|InGameEvent _asgeneric_in_game_event))))))

(event EventBeginPlay
  (Variables|Default|SetCurrentAlive (Utilities|Array|Length (Variables|Default|GetEnemyLocations))))

(event Collision|EventActorBeginOverlap
  (params (OtherActor :type Actor%20Object%20Reference)))

(event EventTick
  (params (DeltaSeconds :type Float%20%28single-precision%29)))

(event EventInGameEvent
  (Development|PrintString "Calling Spawn All Characters")
  (CallFunction|SpawnAllCharacters))

(fn ConstructionScript)

(fn SpawnAllCharacters
  (for (_array_element _array_index) (Variables|Default|GetEnemyLocations)
    (bind _returnvalue (AI|SpawnAIFromClass "/Game/EnemyCharacter/Blueprints/BP_EnemyCharacter.BP_EnemyCharacter_C" "/Game/EnemyCharacter/Blueprints/EnemyAI/BT_EnemyAI.BT_EnemyAI" (+ _array_element (Transformation|GetWorldLocation (Variables|Default|GetDefaultSceneRoot))) "0, 0, 0" false))
    (bind _asbp_enemy_character (Utilities|Casting|CastToBP_EnemyCharacter _returnvalue))
    (if (Variables|Default|GetCompletionIsEvent)
      (EventDispatchers|BindEventtoEnemyDead _asbp_enemy_character (EventDispatchers|CreateEvent :!event Custom|TriggerAllKilledEvent)))
    (if (Variables|Default|GetSpawnPlayerAware)
      (Default|InitializeAwareOfPlayer _asbp_enemy_character)
      (else
        (Default|Initialize _asbp_enemy_character (Utilities|Array|Get(acopy) (Variables|Default|GetVolumeTriggers) _array_index) (Utilities|Array|Get(acopy) (Variables|Default|GetMovementSplines) _array_index))))))