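; BP_EventUseButton is a use trigger that lets the first-person character fire a referenced GenericInGameEvent.
; The first Box overlap by the character binds to its IsUsing event, which calls InGameEvent on that reference if PlayerInRange is true.
; End overlap also sets PlayerInRange to true, so once entered, the trigger keeps responding after the player leaves.
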(event OnComponentBeginOverlap(Box)
  (params (OverlappedComponent :type Primitive%20Component%20Object%20Reference) (OtherActor :type Actor%20Object%20Reference) (OtherComp :type Primitive%20Component%20Object%20Reference) (OtherBodyIndex :type Integer) (bFromSweep :type Boolean) (SweepResult :type Hit%20Result%20Structure%20%28by%20ref%29))
  (bind _asfirst_person_character (Utilities|Casting|CastToFirstPersonCharacter OtherActor))
  (Variables|Default|SetPlayerInRange true)
  (if (Variables|Default|GetFirstCollision)
    (EventDispatchers|BindEventtoIsUsing _asfirst_person_character (delegate Custom|UseGenericInGameEvent))
    (Variables|Default|SetFirstCollision false)))

(event OnComponentEndOverlap(Box)
  (params (OverlappedComponent :type Primitive%20Component%20Object%20Reference) (OtherActor :type Actor%20Object%20Reference) (OtherComp :type Primitive%20Component%20Object%20Reference) (OtherBodyIndex :type Integer))
  (Utilities|Casting|CastToFirstPersonCharacter OtherActor)
  (Variables|Default|SetPlayerInRange true))

(event Custom|UseGenericInGameEvent
  (if (Variables|Default|GetPlayerInRange)
    (bind _asgeneric_in_game_event (Utilities|Casting|CastToGenericInGameEvent (Variables|Default|GetGenericInGameEvent)))
    (Default|InGameEvent _asgeneric_in_game_event)))

(event EventBeginPlay)

(event Collision|EventActorBeginOverlap
  (params (OtherActor :type Actor%20Object%20Reference)))

(event EventTick
  (params (DeltaSeconds :type Float%20%28single-precision%29)))

(fn ConstructionScript)