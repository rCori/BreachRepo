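; Enemy character that carries an SKS rifle on a hand socket, shoots at the player and dies from player projectile hits.
; BeginPlay and the two Initialize functions broadcast StartAI, with Initialize also assigning a trigger box and movement spline.
; FireGun spawns a projectile from the muzzle toward the player, with sound and montage.
; Hits subtract health with a headshot bonus; death stops AI logic, plays a random montage, broadcasts EnemyDead and destroys the actor.
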(event Custom|FireGun
  (Variables|Default|SetIsFiring true)
  (bind _asbp_enemy_sks (Utilities|Casting|CastToBP_Enemy_SKS (Variables|/Script/Engine.ChildActorComponent|GetChildActor (Variables|Default|GetGunActor))))
  (Game|SpawnActorfromClass "/Game/BlueprintSource/BP_EnemyProjectile.BP_EnemyProjectile_C" (Math|Transform|MakeTransform (Transformation|GetWorldLocation (Variables|/Game/IBWP3DAssaultRiflePack/Weapons/SKS/BP_Enemy_SKS.BP_Enemy_SKS_C|GetMuzzlePoint _asbp_enemy_sks)) (Math|Rotator|FindLookatRotation (Transformation|GetWorldLocation (Variables|/Game/IBWP3DAssaultRiflePack/Weapons/SKS/BP_Enemy_SKS.BP_Enemy_SKS_C|GetMuzzlePoint _asbp_enemy_sks)) (Transformation|GetActorLocation (Game|Player|GetPlayerPawn 0)))) "AlwaysSpawn" 0 0)
  (Audio|PlaySoundatLocation "/Game/Audio/SFX/MySounds/gun_machinegun_auto_heavy_shot_00_last_with_tail_01_Cue.gun_machinegun_auto_heavy_shot_00_last_with_tail_01_Cue" (Transformation|GetWorldLocation (Variables|/Game/IBWP3DAssaultRiflePack/Weapons/SKS/BP_Enemy_SKS.BP_Enemy_SKS_C|GetMuzzlePoint _asbp_enemy_sks)))
  (Animation|PlayAnimMontage "/Game/SkeletonMeshes/EnemyCharacter/Animations/HeavyG_Fire_Rifle_Ironsights_Montage.HeavyG_Fire_Rifle_Ironsights_Montage" 0.85 "None"))

(event Custom|EnemyDie
  (AI|Logic|StopLogic (Variables|/Script/AIModule.AIController|GetBrainComponent (AI|GetAIController self)) "")
  (switch int (Math|Random|RandomIntegerinRange 0 2)
    (:0
      (bind _returnvalue (Animation|PlayAnimMontage "/Game/SkeletonMeshes/EnemyCharacter/Animations/HeavyG_Death_1_Montage.HeavyG_Death_1_Montage" 1.0 "None"))
      (Utilities|FlowControl|Delay _returnvalue))
    (:1
      (bind _returnvalue_2 (Animation|PlayAnimMontage "/Game/SkeletonMeshes/EnemyCharacter/Animations/HeavyG_Death_2_Montage.HeavyG_Death_2_Montage" 1.0 "None"))
      (Utilities|FlowControl|Delay _returnvalue_2))
    (:2
      (bind _returnvalue_3 (Animation|PlayAnimMontage "/Game/SkeletonMeshes/EnemyCharacter/Animations/HeavyG_Death_3_Montage.HeavyG_Death_3_Montage" 1.0 "None"))
      (Utilities|FlowControl|Delay _returnvalue_3)))
  (Default|CallEnemyDead)
  (Actor|DestroyActor))

(event Custom|StopFiring
  (Variables|Default|SetIsFiring false))

(event EventBeginPlay
  (if (and (Utilities|IsValid (Variables|Default|GetBP_VolumeTrigger)) (Utilities|IsValid (Variables|Default|GetBP_MoveSplineComponent)))
    (Default|CallStartAI)))

(event Collision|EventActorBeginOverlap
  (params (OtherActor :type Actor%20Object%20Reference)))

(event EventTick
  (params (DeltaSeconds :type Float%20%28single-precision%29)))

(event Collision|EventHit
  (params (MyComp :type Primitive%20Component%20Object%20Reference) (Other :type Actor%20Object%20Reference) (OtherComp :type Primitive%20Component%20Object%20Reference) (bSelfMoved :type Boolean) (HitLocation :type Vector :default "0, 0, 0") (HitNormal :type Vector :default "0, 0, 0") (NormalImpulse :type Vector :default "0, 0, 0") (Hit :type Hit%20Result%20Structure%20%28by%20ref%29))
  (bind _asfirst_person_projectile (Utilities|Casting|CastToFirstPersonProjectile Other))
  (bind _damagegiven (Default|GetDamageGiven _asfirst_person_projectile))
  (Default|CallEnemyHit)
  (Effects|SpawnEmitteratLocation "/Game/Particles/GunShot_Blood.GunShot_Blood" HitLocation)
  (Actor|DestroyActor _asfirst_person_projectile)
  (if (not (Variables|Default|GetHasDied))
    (if (== MyComp (Variables|Default|GetHeadBox))
      (Variables|Default|SetHealth (- (Variables|Default|GetHealth) (* _damagegiven 1.25)))
      (else
        (Variables|Default|SetHealth (- (Variables|Default|GetHealth) _damagegiven))))
    (if (<= (Variables|Default|GetHealth) 0.0)
      (Variables|Default|SetHasDied true)
      (CallFunction|EnemyDie))))

(fn ConstructionScript
  (bind _returnvalue (AddComponent|AddChildActorComponent true))
  (bind _output_get (Variables|Default|SetGunActor _returnvalue))
  (Transformation|AttachComponentToComponent _output_get (Variables|Character|GetMesh) "SKS_right_hand_socket" "KeepRelative" "KeepRelative" "KeepRelative" true))

(fn Initialize
  (params (TriggerBox :type Trigger%20Box%20Object%20Reference) (MoveSpline :type BP%20Movement%20Spline%20Object%20Reference))
  (Default|SetTriggerBox (Variables|Default|GetBP_VolumeTrigger) TriggerBox)
  (Default|SetMovementSpline (Variables|Default|GetBP_MoveSplineComponent) MoveSpline)
  (Default|CallStartAI))

(fn InitializeAwareOfPlayer
  (Default|CallStartAI))