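; BP_MovementSpline is a spline path actor that supplies successive world-space waypoints, apparently for enemy character movement.
; The construction script caches the spline's point count.
; GetNextLocation steps a stored index along the points, reversing at either end for a ping-pong route, and returns that point's location.
; Index and direction live on the spline actor, and its event graph has no active logic.
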(event EventBeginPlay)

(event Collision|EventActorBeginOverlap
  (params (OtherActor :type Actor%20Object%20Reference)))

(event EventTick
  (params (DeltaSeconds :type Float%20%28single-precision%29)))

(fn ConstructionScript
  (Variables|Default|SettotalSplinePoints (Spline|GetNumberOfSplinePoints (Variables|Default|GetSpline))))

(fn GetNextLocation
  (if (Variables|Default|GetinReverse)
    (if (== (Variables|Default|GetcurrentIndex) 0)
      (Variables|Default|SetinReverse false)
      (Math|Integer|IncrementInt (Variables|Default|GetcurrentIndex)
        (:%20%20
          _))
      (else
        (Math|Integer|DecrementInt (Variables|Default|GetcurrentIndex)
          (:%20%20
            _))))
    (elif (== (Variables|Default|GetcurrentIndex) (- (Variables|Default|GettotalSplinePoints) 1))
      (Variables|Default|SetinReverse true)
      (Math|Integer|DecrementInt (Variables|Default|GetcurrentIndex)
        (:%20%20
          _))
      (else
        (Math|Integer|IncrementInt (Variables|Default|GetcurrentIndex)
          (:%20%20
            _)))))
  (return (Spline|GetLocationatSplinePoint (Variables|Default|GetSpline) (Variables|Default|GetcurrentIndex) "World")))