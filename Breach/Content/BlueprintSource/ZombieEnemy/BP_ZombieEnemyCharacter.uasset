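; BP_ZombieEnemyCharacter is a zombie enemy character that takes damage from first-person projectiles and tracks its death.
; A hit on its HitBox spawns a blood effect, destroys the projectile and, while alive, lowers Health by a fixed one point; the projectile's damage subtraction is disconnected.
; At zero health it only sets HasDied and prints a message.
; GetIsAttackRange exposes an attack-range flag that nothing here sets.
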(event EventBeginPlay)

(event Collision|EventActorBeginOverlap
  (params (OtherActor :type Actor%20Object%20Reference)))

(event EventTick
  (params (DeltaSeconds :type Float%20%28single-precision%29)))

(event Collision|EventHit
  (params (MyComp :type Primitive%20Component%20Object%20Reference) (Other :type Actor%20Object%20Reference) (OtherComp :type Primitive%20Component%20Object%20Reference) (bSelfMoved :type Boolean) (HitLocation :type Vector :default "0, 0, 0") (HitNormal :type Vector :default "0, 0, 0") (NormalImpulse :type Vector :default "0, 0, 0") (Hit :type Hit%20Result%20Structure%20%28by%20ref%29))
  (if (== MyComp (Variables|Default|GetHitBox))
    (bind _asfirst_person_projectile (Utilities|Casting|CastToFirstPersonProjectile Other))
    (bind _damagegiven (Default|GetDamageGiven _asfirst_person_projectile))
    (Effects|SpawnEmitteratLocation "/Game/Particles/GunShot_Blood.GunShot_Blood" HitLocation)
    (Actor|DestroyActor _asfirst_person_projectile)
    (if (not (Variables|Default|GetHasDied))
      (Variables|Default|SetHealth (- (Variables|Default|GetHealth) 1.0))
      (if (<= (Variables|Default|GetHealth) 0.0)
        (Variables|Default|SetHasDied true)
        (Development|PrintString "Zombie died")))))

(fn ConstructionScript)

(fn GetIsAttackRange
  (return (Variables|Default|GetisAttackRange)))