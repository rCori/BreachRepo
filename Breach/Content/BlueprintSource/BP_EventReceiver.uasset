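; BP_EventReceiver is an actor that shows and removes a waypoint marker for its event tag.
; Its CreateWaypointWidget and RemoveWaypointWidget functions cast the game mode to CPP_FirstPersonGameMode and delegate to it, passing the actor, EventTag and WaypointOffset on creation and just the tag on removal.
; The event graph and construction script are empty, so these functions run only when called from elsewhere, such as a subclass or another object.
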(event EventBeginPlay)

(event Collision|EventActorBeginOverlap
  (params (OtherActor :type Actor%20Object%20Reference)))

(event EventTick
  (params (DeltaSeconds :type Float%20%28single-precision%29)))

(fn ConstructionScript)

(fn CreateWaypointWidget
  (bind _ascpp_first_person_game_mode (Utilities|Casting|CastToCPP_FirstPersonGameMode (Game|GetGameMode)))
  (Class|CPPFirstPersonGameMode|CreateWaypoint _ascpp_first_person_game_mode self (Variables|Default|GetEventTag) (Variables|Default|GetWaypointOffset)))

(fn RemoveWaypointWidget
  (bind _ascpp_first_person_game_mode (Utilities|Casting|CastToCPP_FirstPersonGameMode (Game|GetGameMode)))
  (Default|RemoveWaypoint _ascpp_first_person_game_mode (Variables|Default|GetEventTag)))