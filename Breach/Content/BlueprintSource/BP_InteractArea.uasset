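; BP_InteractArea is an interaction area that lets the first-person player trigger an interaction while in range.
; On BeginPlay it listens to its in-range dispatcher, then binds to or unbinds from the controlled FirstPersonCharacter's IsUsing dispatcher as range changes.
; A custom event calls DoInteraction, whose logic is not defined in these graphs.
; The unbind path reuses the character reference cast on entry, and no Tick polling is used.
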(event Custom|BindToPlayerInteract
  (params (IsInRange :type Boolean))
  (if IsInRange
    (bind _asfirst_person_character (Utilities|Casting|CastToFirstPersonCharacter (Pawn|GetControlledPawn (Game|GetPlayerController 0))))
    (EventDispatchers|BindEventtoIsUsing _asfirst_person_character (EventDispatchers|CreateEvent :!event Custom|MyCustom))
    (else
      (EventDispatchers|UnbindEventfromIsUsing _asfirst_person_character (EventDispatchers|CreateEvent :!event Custom|MyCustom)))))

(event Custom|MyCustom
  (Class|InteractArea|DoInteraction))

(event EventBeginPlay
  (EventDispatchers|BindEventtoIsinRangeInteract (delegate Custom|BindToPlayerInteract)))

(event Collision|EventActorBeginOverlap
  (params (OtherActor :type Actor%20Object%20Reference)))

(event EventTick
  (params (DeltaSeconds :type Float%20%28single-precision%29)))

(fn ConstructionScript)