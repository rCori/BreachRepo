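; Hinged door that the player toggles with the use input while in range, or that shows an on-screen message when locked.
; The trigger volume binds to the character's use event on first overlap; timelines swing the mesh's yaw to open or close it.
; An overridden in-game event can unlock it, announcing this and creating a waypoint through the C++ game mode.
; The waypoint is removed once the door finishes opening.
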(event OnComponentBeginOverlap(PlayerActivateVolume)
  (params (OverlappedComponent :type Primitive%20Component%20Object%20Reference) (OtherActor :type Actor%20Object%20Reference) (OtherComp :type Primitive%20Component%20Object%20Reference) (OtherBodyIndex :type Integer) (bFromSweep :type Boolean) (SweepResult :type Hit%20Result%20Structure%20%28by%20ref%29))
  (bind _asfirst_person_character (Utilities|Casting|CastToFirstPersonCharacter OtherActor))
  (Variables|Default|SetPlayerInRange true)
  (if (Variables|Default|GetFirstCollision)
    (EventDispatchers|BindEventtoIsUsing _asfirst_person_character (delegate Custom|ToggleUnlockedDoor))
    (Variables|Default|SetFirstCollision false)))

(event OnComponentEndOverlap(PlayerActivateVolume)
  (params (OverlappedComponent :type Primitive%20Component%20Object%20Reference) (OtherActor :type Actor%20Object%20Reference) (OtherComp :type Primitive%20Component%20Object%20Reference) (OtherBodyIndex :type Integer))
  (Utilities|Casting|CastToFirstPersonCharacter OtherActor)
  (Variables|Default|SetPlayerInRange false))

(event Custom|ToggleUnlockedDoor
  (if (Variables|Default|GetPlayerInRange)
    (if (not (Variables|Default|GetIsLocked))
      (Class|CPPDoor|ToggleDoor)
      (else
        (bind _ascpp_first_person_game_mode (Utilities|Casting|CastToCPP_FirstPersonGameMode (Game|GetGameMode)))
        (Default|CallChangeonScreenMessage _ascpp_first_person_game_mode "Door is locked" 2.0)))))

(event EventBeginPlay)

(event Collision|EventActorBeginOverlap
  (params (OtherActor :type Actor%20Object%20Reference)))

(event EventTick
  (params (DeltaSeconds :type Float%20%28single-precision%29)))

(event EventCloseDoor
  (bind _doortrack (Timeline|DoorClose PlayFromStart)
    (:Update
      (Transformation|SetRelativeRotation (Variables|Default|GetDoorMesh) (Math|Rotator|MakeRotator 0.0 0.0 (Math|Float|Lerp 9e+01 0.0 _doortrack)) false false))
    (:Finished
      (Variables|Default|SetIsOpen false))))

(event EventOpenDoor
  (bind _doortrack (Timeline|DoorOpening PlayFromStart)
    (:Update
      (Transformation|SetRelativeRotation (Variables|Default|GetDoorMesh) (Math|Rotator|MakeRotator 0.0 0.0 (Math|Float|Lerp 0.0 9e+01 _doortrack)) false false))
    (:Finished
      (Variables|Default|SetIsOpen true)
      (CallFunction|RemoveWaypointWidget))))

(event EventInGameEvent
  ;[1 1 1] I AM ASSUMING that Parent: In Game Event is my CPP implementation
  (|CallParentFunction)
  (if (Variables|Default|GetUnlocksOnEvent)
    (Variables|Default|SetIsLocked false)
    (bind _ascpp_first_person_game_mode (Utilities|Casting|CastToCPP_FirstPersonGameMode (Game|GetGameMode)))
    (Default|CallChangeonScreenMessage _ascpp_first_person_game_mode "A door has been unlocked" 2.0)
    (CallFunction|CreateWaypointWidget)))

(fn ConstructionScript)

(fn CreateWaypointWidget
  (bind _ascpp_first_person_game_mode (Utilities|Casting|CastToCPP_FirstPersonGameMode (Game|GetGameMode)))
  (Class|CPPFirstPersonGameMode|CreateWaypoint _ascpp_first_person_game_mode self (Variables|Default|GetEventTag) (Variables|Default|GetWaypointOffset)))

(fn RemoveWaypointWidget
  (bind _ascpp_first_person_game_mode (Utilities|Casting|CastToCPP_FirstPersonGameMode (Game|GetGameMode)))
  (Default|RemoveWaypoint (stale _asfirst_person_game_mode) (Variables|Default|GetEventTag)))