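; BP_VolumeTrigger watches an assigned TriggerBox and records when the first-person player character enters it.
; It binds to the box's actor begin-overlap event on BeginPlay if the box is valid, or when SetTriggerBox assigns one at runtime.
; The overlap handler ignores other actors, sets the TriggerEntered flag for the player and prints a debug message; nothing here resets the flag.
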(event Custom|OnTriggerOverlap
  (params (OverlappedActor :type Actor%20Object%20Reference) (OtherActor :type Actor%20Object%20Reference))
  (Utilities|Casting|CastToFirstPersonCharacter OtherActor)
  (Variables|Default|SetTriggerEntered true)
  (Development|PrintString "Trigger was entered"))

(event Custom|SetTriggerBox
  (params (TriggerBox :type Trigger%20Box%20Object%20Reference))
  (bind _output_get (Variables|Default|SetTriggerBox TriggerBox))
  (Collision|BindEventtoOnActorBeginOverlap _output_get (EventDispatchers|CreateEvent :!event Custom|OnTriggerOverlap)))

(event EventBeginPlay
  (bind _triggerbox (Variables|Default|GetTriggerBox))
  (Utilities|IsValid _triggerbox
    (:Is%20Valid
      (Collision|BindEventtoOnActorBeginOverlap _triggerbox (EventDispatchers|CreateEvent :!event Custom|OnTriggerOverlap)))))

(event EventTick
  (params (DeltaSeconds :type Float%20%28single-precision%29)))

(event EventEndPlay
  (params (EndPlayReason :type EEndPlayReason%20Enum :default "Destroyed")))