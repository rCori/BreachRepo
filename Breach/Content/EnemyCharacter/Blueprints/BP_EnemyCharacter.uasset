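; BP_EnemyCharacter is an armed enemy character that shoots projectiles at the player and detects hits from player projectiles.
; Its construction script attaches a child-actor gun to the mesh's right-hand socket.
; FireGun plays a rifle montage and spawns BP_EnemyProjectile at the SKS muzzle, aimed at the player pawn; StopFiring clears the firing flag.
; Capsule hits by FirstPersonProjectile destroy it and only print its damage, without reducing health.
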(event OnComponentBeginOverlap(CapsuleComponent)
  (params (OverlappedComponent :type Primitive%20Component%20Object%20Reference) (OtherActor :type Actor%20Object%20Reference) (OtherComp :type Primitive%20Component%20Object%20Reference) (OtherBodyIndex :type Integer) (bFromSweep :type Boolean) (SweepResult :type Hit%20Result%20Structure%20%28by%20ref%29)))

(event OnComponentHit(CapsuleComponent)
  (params (HitComponent :type Primitive%20Component%20Object%20Reference) (OtherActor :type Actor%20Object%20Reference) (OtherComp :type Primitive%20Component%20Object%20Reference) (NormalImpulse :type Vector :default "0, 0, 0") (Hit :type Hit%20Result%20Structure%20%28by%20ref%29))
  (bind _asfirst_person_projectile (Utilities|Casting|CastToFirstPersonProjectile OtherActor))
  (bind _newparam (Default|GetDamageGiven _asfirst_person_projectile))
  (Actor|DestroyActor _asfirst_person_projectile)
  (Development|PrintString (Utilities|String|ToString(Text) (Utilities|Text|FormatText "Enemy takes {damageAmount} damage" _newparam)) true true "(R=0.001685,G=1.000000,B=0.000000,A=1.000000)"))

(event Custom|FireGun
  (Variables|Default|SetIsFiring true)
  (Animation|Montage|PlayMontage (Variables|Character|GetMesh) "/Game/EnemyCharacter/Mannequin/Animations/HeavyG_Fire_Rifle_Ironsights_Montage.HeavyG_Fire_Rifle_Ironsights_Montage"
    (:then
      (Development|PrintString "Enemy is firing gun" true true "(R=1.000000,G=0.000000,B=0.000000,A=1.000000)")
      (bind _asbp_enemy_sks (Utilities|Casting|CastToBP_Enemy_SKS (Variables|/Script/Engine.ChildActorComponent|GetChildActor (Variables|Default|GetGunActor))))
      (Game|SpawnActorfromClass "/Game/FirstPersonBP/Blueprints/BP_EnemyProjectile.BP_EnemyProjectile_C" (Math|Transform|MakeTransform (Transformation|GetWorldLocation (Variables|/Game/IBWP3DAssaultRiflePack/Weapons/SKS/BP_Enemy_SKS.BP_Enemy_SKS_C|GetMuzzlePoint _asbp_enemy_sks)) (Math|Rotator|FindLookatRotation (Transformation|GetWorldLocation (Variables|/Game/IBWP3DAssaultRiflePack/Weapons/SKS/BP_Enemy_SKS.BP_Enemy_SKS_C|GetMuzzlePoint _asbp_enemy_sks)) (Transformation|GetActorLocation (Game|Player|GetPlayerPawn 0))) "1,1.000000,1") "AlwaysSpawn" 0 0))))

(event Custom|StopFiring
  (Variables|Default|SetIsFiring false))

(event EventBeginPlay)

(event Collision|EventActorBeginOverlap
  (params (OtherActor :type Actor%20Object%20Reference)))

(event EventTick
  (params (DeltaSeconds :type Float%20%28single-precision%29)))

(fn ConstructionScript
  (bind _returnvalue (AddComponent|AddChildActorComponent true))
  (bind _output_get (Variables|Default|SetGunActor _returnvalue))
  (Transformation|AttachComponentToComponent _output_get (Variables|Character|GetMesh) "SKS_right_hand_socket" "KeepRelative" "KeepRelative" "KeepRelative" true))