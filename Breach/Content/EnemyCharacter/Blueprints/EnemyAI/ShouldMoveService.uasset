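; Behavior tree service for enemy AI that randomly decides on a repositioning move relative to the player's stored location.
; Each tick it rolls among three outcomes: shift toward or away from the player, strafe sideways via a cross product with the up vector, or do nothing.
; Either move writes the next location to the Blackboard and sets the random-movement flag, which this service never clears.
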(event EventReceiveTickAI
  (params (OwnerController :type AI%20Controller%20Object%20Reference) (ControlledPawn :type Pawn%20Object%20Reference) (DeltaSeconds :type Float%20%28single-precision%29))
  (bind _returnvalue (Transformation|GetActorLocation ControlledPawn))
  (bind _bbks_playerlocation (Variables|Default|GetBBKS_PlayerLocation))
  (bind _returnvalue_2 (Class|BTFunctionLibrary|GetBlackboardValueasVector _bbks_playerlocation))
  (bind _returnvalue_3 (- _returnvalue _returnvalue_2))
  (bind _returnvalue_4 (Math|Vector|Normalize _returnvalue_3))
  (switch int (Math|Random|RandomIntegerinRange 0 2)
    (:0
      (AI|BehaviorTree|SetBlackboardValueasVector (Variables|Default|GetBBKS_NextLocation) (+ (* _returnvalue_4 (Math|Random|RandomFloatinRange -2e+02 2e+02)) _returnvalue)))
    (:1
      (AI|BehaviorTree|SetBlackboardValueasVector (Variables|Default|GetBBKS_NextLocation) (+ (* (Math|Vector|CrossProduct "0, 0,1.000000" _returnvalue_4) (Math|Random|RandomFloatinRange -5e+02 5e+02)) _returnvalue))))
  (Class|BTFunctionLibrary|SetBlackboardValueasBool (Variables|Default|GetBBKS_ShouldDoRandomMovement) true))