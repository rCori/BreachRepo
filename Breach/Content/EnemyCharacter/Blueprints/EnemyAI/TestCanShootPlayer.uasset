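; Behavior tree task that tests whether an enemy AI pawn has a shot on the player.
; When the blackboard player location is within an accepted distance, it line-traces to that location, ignoring itself, with debug drawing.
; It succeeds and clears the shot-blocked blackboard flag if the trace hits the player's pawn.
; Otherwise, including when out of range, it sets the flag and fails.
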(event EventReceiveExecuteAI
  (params (OwnerController :type AI%20Controller%20Object%20Reference) (ControlledPawn :type Pawn%20Object%20Reference))
  (bind _returnvalue (Transformation|GetActorLocation ControlledPawn))
  (bind _bbks_playerlocation (Variables|Default|GetBBKS_PlayerLocation))
  (bind _returnvalue_2 (Class|BTFunctionLibrary|GetBlackboardValueasVector _bbks_playerlocation))
  (if (<= (Math|Vector|VectorLength (- _returnvalue _returnvalue_2)) (Variables|Default|GetAcceptedDistance))
    (bind _outhit (Collision|LineTraceByChannel _returnvalue _returnvalue_2 "TraceTypeQuery3" false (Utilities|Array|MakeArray ControlledPawn) (Variables|Default|GetTraceDebug)))
    (if (== (.HitActor (Collision|BreakHitResult _outhit)) (Pawn|GetControlledPawn (Game|GetPlayerController 0)))
      (Development|PrintString "Enemy has shot on player")
      (Class|BTFunctionLibrary|SetBlackboardValueasBool (Variables|Default|GetBBKS_IsShotBlocked) false)
      (AI|BehaviorTree|FinishExecute true)
      (else
        (Class|BTFunctionLibrary|SetBlackboardValueasBool (Variables|Default|GetBBKS_IsShotBlocked) true)
        (AI|BehaviorTree|FinishExecute false)))
    (else
      (Development|PrintString "Enemy to far away from player to shoot")
      (Class|BTFunctionLibrary|SetBlackboardValueasBool (Variables|Default|GetBBKS_IsShotBlocked) true)
      (AI|BehaviorTree|FinishExecute false))))