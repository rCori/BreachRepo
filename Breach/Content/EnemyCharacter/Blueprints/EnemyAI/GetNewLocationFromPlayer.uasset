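; Behavior tree task that picks a standoff move-to point for an enemy near the player and writes it to the blackboard.
; It line-traces from the stored player location to the controlled pawn, ignoring the player.
; If the hit is at least MinimumDistance away, the point sits that far from the player toward the pawn; otherwise it uses the hit location.
; Debug trace and prints are active, with both branches printing "greater than".
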(event EventReceiveExecuteAI
  (params (OwnerController :type AI%20Controller%20Object%20Reference) (ControlledPawn :type Pawn%20Object%20Reference))
  (bind _returnvalue (Transformation|GetActorLocation ControlledPawn))
  (bind _bbks_playerlocation (Variables|Default|GetBBKS_PlayerLocation))
  (bind _minimumdistance (Variables|Default|GetMinimumDistance))
  (bind _bbks_newlocation (Variables|Default|GetBBKS_NewLocation))
  (bind _returnvalue_2 (Class|BTFunctionLibrary|GetBlackboardValueasVector _bbks_newlocation))
  (bind _returnvalue_3 (Class|BTFunctionLibrary|GetBlackboardValueasVector _bbks_playerlocation))
  (Variables|Default|SetDifferenceVec (- _returnvalue_3 _returnvalue))
  (bind _outhit (Collision|LineTraceByChannel _returnvalue_3 _returnvalue "TraceTypeQuery3" false (Utilities|Array|MakeArray (Game|Player|GetPlayerPawn 0)) (Variables|Default|GetTraceDebug) true "(R=0.000000,G=0.039997,B=1.000000,A=1.000000)" "(R=1.000000,G=0.000000,B=0.582807,A=1.000000)"))
  (if (>= (.Distance (Collision|BreakHitResult _outhit)) _minimumdistance)
    (AI|BehaviorTree|SetBlackboardValueasVector _bbks_newlocation (- _returnvalue_3 (* (Math|Vector|Normalize (Variables|Default|GetDifferenceVec)) (Variables|Default|GetMinimumDistance))))
    (Development|PrintString (Utilities|String|ToString(Text) (Utilities|Text|FormatText "Distance was greater than {distance} 
MoveTo position is ({x}, {y}, {z})" _minimumdistance (.x _returnvalue_2) (.y _returnvalue_2) (.z _returnvalue_2))))
    (else
      (AI|BehaviorTree|SetBlackboardValueasVector _bbks_newlocation (.Location (Collision|BreakHitResult _outhit)))
      (Development|PrintString (Utilities|String|ToString(Text) (Utilities|Text|FormatText "Distance was greater than {distance} 
MoveTo position is ({x}, {y}, {z})" _minimumdistance (.x _returnvalue_2) (.y _returnvalue_2) (.z _returnvalue_2))))))
  (AI|BehaviorTree|FinishExecute true))